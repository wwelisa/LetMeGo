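; Base arrow actor that serves as a pickup, bow ammo and projectile, driven by a small enter/exit state machine (Unobtained, In Bow, In Air).
; Fire creates a temporary projectile movement component with speed scaled by bow charge, destroyed when flight ends.
; Hitting anything but the player embeds the arrow by charge-based depth, attaches it and makes it Unobtained.
; Player overlap then adds its kind to the game mode and destroys it.
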(event `self.ReceiveBeginPlay`
  (bind _asbp_game_mode_let_me_go (cast `/Game/Blueprints/BP_GameMode_LetMeGo` (`GameplayStatics.GetGameMode`)))
  (set `self.Game Mode Let Me Go` _asbp_game_mode_let_me_go))

(event `Fire`
  (params (BowCharge :type "Float (double-precision)"))
  (set `self.Bow Charge` BowCharge)
  (`self.SetArrowState` "NewEnumerator3"))

(event `self.Arrow.OnComponentBeginOverlap`
  (params (OverlappedComponent :type "PrimitiveComponent Object Reference") (OtherActor :type "Actor Object Reference") (OtherComp :type "PrimitiveComponent Object Reference") (OtherBodyIndex :type Integer) (bFromSweep :type Boolean) (SweepResult :type "HitResult Structure (by ref)"))
  (`self.HandleOverlap` OtherActor SweepResult))

(fn `HandleOverlap`
  (params (OtherActor :type "Actor Object Reference") (HitResult :type "HitResult Structure"))
  (bind (_hitresult_bblockinghit _hitresult_binitialoverlap _hitresult_time _hitresult_distance _hitresult_location _hitresult_impactpoint) (`GameplayStatics.BreakHitResult` (`local.HitResult`)))
  (switch `/Game/Geometry/Meshes/Arrow/E_Arrowstate` (`self.ArrowState`)
    (:`NewEnumerator1`
      (cast `/Game/FirstPersonBP/Blueprints/FirstPersonCharacter` (`local.OtherActor`))
      (`/Game/Blueprints/BP_GameMode_LetMeGo.AddArrow` (`self.Game Mode Let Me Go`) (`self.ArrowKind`))
      (`self.K2_DestroyActor`))
    (:`NewEnumerator3`
      (if (!= (`local.OtherActor`) (`GameplayStatics.GetPlayerCharacter` 0))
        (`self.SetArrowState` "NewEnumerator1")
        (`self.K2_SetActorLocation` (- _hitresult_impactpoint (* (`self.GetActorForwardVector`) (`KismetMathLibrary.Lerp` 55.0 30.0 (`self.Bow Charge`)))))
        (`self.K2_AttachToActor` (`local.OtherActor`) "None" "KeepWorld" "KeepWorld" "KeepWorld")))))

(fn `OnStateBeginn`
  (params (State :type "/Game/Geometry/Meshes/Arrow/E_Arrowstate Enum" :default "NewEnumerator0"))
  (switch `/Game/Geometry/Meshes/Arrow/E_Arrowstate` State
    (:`NewEnumerator1`
      (`PrimitiveComponent.SetCollisionProfileName` (`self.Arrow`) "OverlapAllDynamic" true))
    (:`NewEnumerator2`
      (`PrimitiveComponent.SetCollisionProfileName` (`self.Arrow`) "NoCollision" true))
    (:`NewEnumerator3`
      (`PrimitiveComponent.SetCollisionProfileName` (`self.Arrow`) "OverlapAllDynamic" true)
      (bind _returnvalue (`AddComponent|NODE_AddProjectileMovementComponent-0`))
      (bind _output_get (set `self.ProjectileComponent` _returnvalue))
      (set `MovementComponent.Velocity` (* (`self.GetActorForwardVector`) (`KismetMathLibrary.Lerp` 100.0 4000.0 (`self.Bow Charge`))) _output_get)
      (set `ProjectileMovementComponent.bRotationFollowsVelocity` true _output_get))))

(fn `OnStateEnd`
  (params (State :type "/Game/Geometry/Meshes/Arrow/E_Arrowstate Enum" :default "NewEnumerator0"))
  (switch `/Game/Geometry/Meshes/Arrow/E_Arrowstate` State
    (:`NewEnumerator3`
      (`ActorComponent.K2_DestroyComponent` (`self.ProjectileComponent`)))))

(fn `SetArrowState`
  (params (NewState :type "/Game/Geometry/Meshes/Arrow/E_Arrowstate Enum" :default "NewEnumerator0"))
  (if (`|EnumInequality` NewState (`self.ArrowState`))
    (`self.OnStateEnd` (`self.ArrowState`)) ; Leave Current state
    (bind _output_get (set `self.ArrowState` (`local.NewState`)))
    (`self.OnStateBeginn` _output_get) ; enter new state
  ))

(fn `UserConstructionScript`)