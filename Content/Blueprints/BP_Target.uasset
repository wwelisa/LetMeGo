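; BP_Target is a shootable target that reacts the first time a FirstPersonProjectile hits its static mesh.
; The mesh's hit event casts the other actor to the projectile and uses the IsHit flag to ignore later hits.
; It then turns on physics simulation, launching the mesh along the hit normal with a velocity-change impulse and adding torque around its forward vector.
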(event `self.StaticMesh.OnComponentHit`
  (params (HitComponent :type "PrimitiveComponent Object Reference") (OtherActor :type "Actor Object Reference") (OtherComp :type "PrimitiveComponent Object Reference") (NormalImpulse :type "Vector Structure") (Hit :type "HitResult Structure (by ref)"))
  (bind _staticmesh (`self.StaticMesh`))
  ;[1 1 1] Change for Projektile
  (cast `/Game/FirstPersonBP/Blueprints/FirstPersonProjectile` OtherActor)
  (if (not (`self.IsHit?`))
    (set `self.IsHit?` true)
    (`PrimitiveComponent.SetSimulatePhysics` _staticmesh true)
    (`PrimitiveComponent.AddImpulse` _staticmesh (* (`.Normal` (`GameplayStatics.BreakHitResult` Hit)) 1000.0) "None" true)
    (`PrimitiveComponent.AddTorqueInRadians` _staticmesh (* (`SceneComponent.GetForwardVector` (`self.StaticMesh`)) 1000.0) "None" true)))

(fn `UserConstructionScript`)