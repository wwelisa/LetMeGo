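; Game mode for LetMeGo that holds the player's slot-based item inventory and Basic and Ice arrow counts.
; It creates WBP_UI on BeginPlay and updates its selection and icons as slots are cycled, filled or cleared.
; AddItem fills the selected slot or searches for a free one, returning an InventoryFull flag.
; ReloadArrow reloads a bow only when it holds neither arrow type.
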(event `self.ReceiveBeginPlay`
  (bind _returnvalue (`|CreateWidget` "/Game/Blueprints/WBP_UI.WBP_UI_C"))
  (bind _output_get (set `self.UIRef` _returnvalue))
  (`UserWidget.AddToViewport` _output_get 0)
  (`/Game/Blueprints/WBP_UI.SelectItem` _output_get (`self.SelectedIndex`)))

(fn `AddArrow`
  (params (NewArrow :type "/Game/Geometry/Meshes/Arrow/E_ArrowKind Enum" :default "NewEnumerator0"))
  (switch `/Game/Geometry/Meshes/Arrow/E_ArrowKind` NewArrow
    (:`NewEnumerator0`
      (`/Engine/EditorBlueprintResources/StandardMacros.IncrementInt` (`self.BasicArrowNum`)))
    (:`NewEnumerator1`
      (`/Engine/EditorBlueprintResources/StandardMacros.IncrementInt` (`self.IceArrowNum`)))))

(fn `AddItem`
  (params (NewKey :type "/Game/Strucktures/Key_Struc Structure"))
  (returns (`InventoryFull?` :type Boolean))
  (if (`KismetSystemLibrary.IsValidClass` (`.ClassRef_16_44BCBDAE4BB9B75AF55869B037B22FB3` (break `/Game/Strucktures/Key_Struc` (`|GetArrayItem` (`self.InventoryArray`) (`self.SelectedIndex`)))))
    (`self.FindFreeSpot`)
    (`/Game/Blueprints/WBP_UI.SelectItem` (`self.UIRef`) (`self.SelectedIndex`))
    (if (`self.InventoryFull?`)
      (`KismetSystemLibrary.PrintString` "Inventory Full")
      (else
        (`KismetArrayLibrary.Array_Set` (`self.InventoryArray`) (`self.SelectedIndex`) (`local.NewKey`) :!label _label)
        (`/Game/Blueprints/WBP_UI.UpdateImage` (`self.UIRef`) (`self.SelectedIndex`) (`.ItemIcon_12_71D765B048B47BF7FC0DE0A1D8FC48CA` (break `/Game/Strucktures/Key_Struc` (`local.NewKey`))))))
    (else
      (goto _label)))
  (return (`self.InventoryFull?`)))

(fn `FindFreeSpot`
  (for _index (range (+ (`self.MaxInventory`) 1))
    (if (`KismetSystemLibrary.IsValidClass` (`.ClassRef_16_44BCBDAE4BB9B75AF55869B037B22FB3` (break `/Game/Strucktures/Key_Struc` (`|GetArrayItem` (`self.InventoryArray`) _index))))
      (if (== (`self.MaxInventory`) _index)
        (set `self.InventoryFull?` true))
      (else
        (set `self.SelectedIndex` _index)
        (break)))))

(fn `ReloadArrow`
  (params (ArrowKind :type "/Game/Geometry/Meshes/Arrow/E_ArrowKind Enum" :default "NewEnumerator0") (Bow :type "/Game/Blueprints/BP_Bow Object Reference"))
  (`/Game/Blueprints/BP_Bow.IceArrow` Bow
    (:`then`)
    (:`else`
      (`/Game/Blueprints/BP_Bow.BasicArrow` Bow
        (:`then`)
        (:`else`
          (`/Game/Blueprints/BP_Bow.Reload` (`local.Bow`) ArrowKind))))))

(fn `RemoveInventoryItem`
  (`KismetArrayLibrary.Array_Set` (`self.InventoryArray`) (`self.SelectedIndex`))
  (`/Game/Blueprints/WBP_UI.UpdateImage` (`self.UIRef`) (`self.SelectedIndex`) null))

(fn `SelectNextKey`
  (if (not (>= (`self.SelectedIndex`) (`self.MaxInventory`)))
    (bind _result (`/Engine/EditorBlueprintResources/StandardMacros.IncrementInt` (`self.SelectedIndex`))
      (:`  `
        (`/Game/Blueprints/WBP_UI.SelectItem` (`self.UIRef`) _result)))))

(fn `SelectPrevKey`
  (if (not (<= (`self.SelectedIndex`) 0))
    (bind _result (`/Engine/EditorBlueprintResources/StandardMacros.DecrementInt` (`self.SelectedIndex`))
      (:`  `
        (`/Game/Blueprints/WBP_UI.SelectItem` (`self.UIRef`) _result)))))

(fn `UserConstructionScript`)