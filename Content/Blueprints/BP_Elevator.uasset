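; BP_Elevator is a platform that travels along a spline path once its TurnOn event fires.
; TurnOn plays the MovePlatform timeline, whose TravelDistance track scales the spline length to set the mesh's world location.
; At BeginPlay and on each timeline update, the mesh takes roll and yaw from the spline's start with pitch zeroed, so its orientation stays fixed during travel.
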(event `self.ReceiveBeginPlay`
  (bind (_returnvalue_roll _returnvalue_pitch _returnvalue_yaw) (`KismetMathLibrary.BreakRotator` (`SplineComponent.GetRotationAtDistanceAlongSpline` (`self.Spline`) 0.0 "Local")))
  (`SceneComponent.K2_SetRelativeRotation` (`self.StaticMesh`) (`KismetMathLibrary.MakeRotator` _returnvalue_roll 0.0 _returnvalue_yaw) false false))

(event `TurnOn`
  (bind _spline (`self.Spline`))
  (bind (_returnvalue_roll _returnvalue_pitch _returnvalue_yaw) (`KismetMathLibrary.BreakRotator` (`SplineComponent.GetRotationAtDistanceAlongSpline` _spline 0.0 "Local")))
  (bind (_direction _traveldistance) (`Timeline|MovePlatform`)
    (:`Update`
      (`SceneComponent.K2_SetWorldLocation` (`self.StaticMesh`) (`SplineComponent.GetLocationAtDistanceAlongSpline` _spline (* _traveldistance (`SplineComponent.GetSplineLength` (`self.Spline`))) "World") false false)
      (`SceneComponent.K2_SetRelativeRotation` (`self.StaticMesh`) (`KismetMathLibrary.MakeRotator` _returnvalue_roll 0.0 _returnvalue_yaw) false false))))

(fn `UserConstructionScript`)