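; BP_Platforms is a moving platform that travels along a spline and can be briefly halted by ice arrows.
; A timeline started on BeginPlay maps TravelDistance to spline length to position the mesh.
; Rotation is always sampled at the spline's start, with pitch zeroed.
; An overlapping BP_Arrow_Ice spawns a hit particle and stops the timeline, which resumes after a short delay.
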(event `self.ReceiveBeginPlay`
  (bind _spline (`self.Spline`))
  (bind (_returnvalue_roll _returnvalue_pitch _returnvalue_yaw) (`KismetMathLibrary.BreakRotator` (`SplineComponent.GetRotationAtDistanceAlongSpline` _spline 0.0 "Local")))
  (bind (_returnvalue_roll_2 _returnvalue_pitch_2 _returnvalue_yaw_2) (`KismetMathLibrary.BreakRotator` (`SplineComponent.GetRotationAtDistanceAlongSpline` (`self.Spline`) 0.0 "Local")))
  (`SceneComponent.K2_SetRelativeRotation` (`self.Mesh`) (`KismetMathLibrary.MakeRotator` _returnvalue_roll_2 0.0 _returnvalue_yaw_2) false false)
  (bind (_direction _traveldistance) (`Timeline|Timeline_Distance` :!label _label)
    (:`Update`
      (`SceneComponent.K2_SetWorldLocation` (`self.Mesh`) (`SplineComponent.GetLocationAtDistanceAlongSpline` _spline (* _traveldistance (`SplineComponent.GetSplineLength` (`self.Spline`))) "World") false false)
      (`SceneComponent.K2_SetRelativeRotation` (`self.Mesh`) (`KismetMathLibrary.MakeRotator` _returnvalue_roll 0.0 _returnvalue_yaw) false false))))

(event `self.Mesh.OnComponentBeginOverlap`
  (params (OverlappedComponent :type "PrimitiveComponent Object Reference") (OtherActor :type "Actor Object Reference") (OtherComp :type "PrimitiveComponent Object Reference") (OtherBodyIndex :type Integer) (bFromSweep :type Boolean) (SweepResult :type "HitResult Structure (by ref)"))
  (cast `/Game/Blueprints/BP_Arrow_Ice` OtherActor)
  (`GameplayStatics.SpawnEmitterAtLocation` "/Game/FXVarietyPack/Particles/P_ky_hit1.P_ky_hit1" SweepResult_Location)
  (`|ExecutionSequence`
    (:`then_0`
      (goto _label :!via `Stop`))
    (:`then_1`
      (`KismetSystemLibrary.Delay` 1.0)
      (goto _label))))

(fn `UserConstructionScript`)