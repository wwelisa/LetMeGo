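; BP_Arrow_Basic is an arrow projectile that explodes when it hits something in flight.
; HandleOverlap acts only while ArrowState is In Air and ignores the player character.
; On a valid overlap it spawns a half-scale explosion particle at the hit location and destroys itself, with no damage applied in this graph.
; The event graph holds only disabled default nodes.
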(fn `HandleOverlap`
  (params (OtherActor :type "Actor Object Reference") (HitResult :type "HitResult Structure"))
  (bind (_hitresult_bblockinghit _hitresult_binitialoverlap _hitresult_time _hitresult_distance _hitresult_location) (`GameplayStatics.BreakHitResult` (`local.HitResult`)))
  (switch `/Game/Geometry/Meshes/Arrow/E_Arrowstate` (`self.ArrowState`)
    (:`NewEnumerator3`
      (if (!= (`local.OtherActor`) (`GameplayStatics.GetPlayerCharacter` 0))
        (`GameplayStatics.SpawnEmitterAtLocation` "/Game/FXVarietyPack/Particles/P_ky_explosion.P_ky_explosion" _hitresult_location (struct) (0.5 0.5 0.5))
        (`self.K2_DestroyActor`)))))

(fn `UserConstructionScript`
  (`parent.UserConstructionScript`))