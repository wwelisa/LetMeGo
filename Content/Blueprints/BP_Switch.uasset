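; BP_Switch is an interactable switch that turns on a linked Platform, optionally requiring a key from the player's inventory.
; When the FirstPersonCharacter overlaps its Collision, it enables E input, first searching BP_GameMode_LetMeGo's InventoryArray for RequiredKey's class if KeyRequired is set.
; Pressing E removes the matched key by its saved index when one is required, then calls TurnOn on the Platform.
; Input is never disabled afterwards.
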(event `self.Collision.OnComponentBeginOverlap`
  (params (OverlappedComponent :type "PrimitiveComponent Object Reference") (OtherActor :type "Actor Object Reference") (OtherComp :type "PrimitiveComponent Object Reference") (OtherBodyIndex :type Integer) (bFromSweep :type Boolean) (SweepResult :type "HitResult Structure (by ref)"))
  (cast `/Game/FirstPersonBP/Blueprints/FirstPersonCharacter` OtherActor)
  (if (`self.KeyRequired`)
    (bind _arrayindex (`self.CheckKey`))
    (set `self.Array Index` _arrayindex)
    (if (`self.GotKey`)
      (`self.EnableInput` (`GameplayStatics.GetPlayerController` 0) :!label _label))
    (else
      (goto _label))))

(event `Key|E`
  (params (Key :type "Key Structure"))
  (:`Pressed`
    (if (`self.KeyRequired`)
      (`/Game/Blueprints/BP_GameMode_LetMeGo.RemoveInventoryItem` (`self.Game Mode Let Me Go`) (`self.Array Index`))
      (set `self.GotKey` false))
    (`/Game/Blueprints/BP_Elevator.TurnOn` (`self.Platform`))))

(fn `CheckKey`
  (returns (ArrayIndex :type Integer))
  (bind (_requiredkey_name _requiredkey_mesh _requiredkey_itemicon _requiredkey_classref) (break `/Game/Strucktures/Key_Struc` (`self.RequiredKey`)))
  (bind _asbp_game_mode_let_me_go (cast `/Game/Blueprints/BP_GameMode_LetMeGo` (`GameplayStatics.GetGameMode`)))
  (bind _output_get (set `self.Game Mode Let Me Go` _asbp_game_mode_let_me_go))
  (for (_array_element _array_index) (`/Game/Blueprints/BP_GameMode_LetMeGo.InventoryArray` _output_get)
    (if (== (`.ClassRef_16_44BCBDAE4BB9B75AF55869B037B22FB3` (break `/Game/Strucktures/Key_Struc` _array_element)) _requiredkey_classref)
      (set `self.GotKey` true)
      (break)))
  (return _array_index))

(fn `UserConstructionScript`)