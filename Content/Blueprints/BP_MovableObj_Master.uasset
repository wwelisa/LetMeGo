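; Master Blueprint for a movable object that only simulates physics while the first-person player is in one of its trigger volumes.
; X-axis and Y-axis collision components turn on mesh physics when a FirstPersonCharacter begins overlapping and turn it off when the overlap ends.
; Each volume toggles physics independently with no overlap count, so leaving one disables physics even if the player remains in the other.
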(event `self.Y_Axis_Collision.OnComponentEndOverlap`
  (params (OverlappedComponent :type "PrimitiveComponent Object Reference") (OtherActor :type "Actor Object Reference") (OtherComp :type "PrimitiveComponent Object Reference") (OtherBodyIndex :type Integer))
  (cast `/Game/FirstPersonBP/Blueprints/FirstPersonCharacter` OtherActor)
  (`PrimitiveComponent.SetSimulatePhysics` (`self.Mesh`) false))

(event `self.Y_Axis_Collision.OnComponentBeginOverlap`
  (params (OverlappedComponent :type "PrimitiveComponent Object Reference") (OtherActor :type "Actor Object Reference") (OtherComp :type "PrimitiveComponent Object Reference") (OtherBodyIndex :type Integer) (bFromSweep :type Boolean) (SweepResult :type "HitResult Structure (by ref)"))
  (cast `/Game/FirstPersonBP/Blueprints/FirstPersonCharacter` OtherActor)
  (`PrimitiveComponent.SetSimulatePhysics` (`self.Mesh`) true))

(event `self.X_Axis_Collision.OnComponentBeginOverlap`
  (params (OverlappedComponent :type "PrimitiveComponent Object Reference") (OtherActor :type "Actor Object Reference") (OtherComp :type "PrimitiveComponent Object Reference") (OtherBodyIndex :type Integer) (bFromSweep :type Boolean) (SweepResult :type "HitResult Structure (by ref)"))
  (cast `/Game/FirstPersonBP/Blueprints/FirstPersonCharacter` OtherActor)
  (`PrimitiveComponent.SetSimulatePhysics` (`self.Mesh`) true))

(event `self.X_Axis_Collision.OnComponentEndOverlap`
  (params (OverlappedComponent :type "PrimitiveComponent Object Reference") (OtherActor :type "Actor Object Reference") (OtherComp :type "PrimitiveComponent Object Reference") (OtherBodyIndex :type Integer))
  (cast `/Game/FirstPersonBP/Blueprints/FirstPersonCharacter` OtherActor)
  (`PrimitiveComponent.SetSimulatePhysics` (`self.Mesh`) false))

(fn `UserConstructionScript`)