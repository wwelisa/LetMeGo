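; Bow actor that handles charging, firing and reloading of Basic and Ice arrows.
; A timeline drives the charge amount and mirrors it to BP_GameMode_LetMeGo; it can reverse to wind down or stop and reset.
; Reload spawns the chosen arrow type attached to the skeletal mesh's arrow socket.
; Fire detaches the current arrow, launches it with the charge amount, then resets the charge timeline.
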(event `BeginnCharge`
  (bind (_direction _chargeamount) (`Timeline|Charge Timeline` :!label _label)
    (:`Update`
      (set `self.ChargeAmout` _chargeamount)
      (bind _asbp_game_mode_let_me_go (cast `/Game/Blueprints/BP_GameMode_LetMeGo` (`GameplayStatics.GetGameMode`)))
      (set `/Game/Blueprints/BP_GameMode_LetMeGo.BowCharge` (`self.ChargeAmout`) _asbp_game_mode_let_me_go))))

(event `StopCharge`
  (`|ExecutionSequence`
    (:`then_0`
      (goto _label :!via `Stop`))
    (:`then_1`
      (goto _label :!via `SetNewTime`))))

(event `EndCharge`
  (goto _label :!via `Reverse`))

(event `Fire`
  (switch `/Game/Geometry/Meshes/Arrow/E_ArrowKind` (`self.ArrowKind`)
    (:`NewEnumerator0`
      (bind _basicarrow (`self.BasicArrow`)
        (:`then`
          (`self.K2_DetachFromActor` _basicarrow "KeepWorld" "KeepWorld" "KeepWorld")
          (`/Game/Blueprints/BP_Arrow_Master.Fire` (`self.BasicArrow`) (`self.ChargeAmout`))
          (set `self.BasicArrow` null))
        (:`else`)))
    (:`NewEnumerator1`
      (bind _icearrow (`self.IceArrow`)
        (:`then`
          (`self.K2_DetachFromActor` _icearrow "KeepWorld" "KeepWorld" "KeepWorld")
          (`/Game/Blueprints/BP_Arrow_Master.Fire` (`self.IceArrow`) (`self.ChargeAmout`))
          (set `self.IceArrow` null))
        (:`else`))))
  (`self.StopCharge`))

(event `Reload`
  (params (ArrowKind :type "/Game/Geometry/Meshes/Arrow/E_ArrowKind Enum" :default "NewEnumerator0"))
  (switch `/Game/Geometry/Meshes/Arrow/E_ArrowKind` ArrowKind
    (:`NewEnumerator0`
      (bind _returnvalue (`|SpawnActorFromClass` "/Game/Blueprints/BP_Arrow_Basic.BP_Arrow_Basic_C" (`KismetMathLibrary.MakeTransform` (0.0 0.0 0.0) (struct) (2.0 2.0 2.0)) "Undefined" "OverrideRootScale" null null))
      (bind _output_get (set `self.BasicArrow` _returnvalue))
      (`self.K2_AttachToComponent` _output_get (`self.SkeletalMesh`) "ArrowAttachSocket" "SnapToTarget" "SnapToTarget" "KeepWorld" true)
      (set `self.ArrowKind` "NewEnumerator0"))
    (:`NewEnumerator1`
      (bind _returnvalue_2 (`|SpawnActorFromClass` "/Game/Blueprints/BP_Arrow_Ice.BP_Arrow_Ice_C" (`KismetMathLibrary.MakeTransform` (0.0 0.0 0.0) (struct) (2.0 2.0 2.0)) "Undefined" "OverrideRootScale" null null))
      (bind _output_get_2 (set `self.IceArrow` _returnvalue_2))
      (`self.K2_AttachToComponent` _output_get_2 (`self.SkeletalMesh`) "ArrowAttachSocket" "SnapToTarget" "SnapToTarget" "KeepWorld" true)
      (set `self.ArrowKind` "NewEnumerator1"))))

(fn `UserConstructionScript`)